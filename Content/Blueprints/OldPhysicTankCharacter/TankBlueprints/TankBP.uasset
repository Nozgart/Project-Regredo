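; TankBP is the Blueprint for a player-drivable tank, forwarding movement input to its TankMovement component.
; BeginPlay initialises TankMovement with the left and right track references.
; The MoveForward axis drives forward intent, while TurnRight passes both its value and the current forward axis so turning accounts for throttle.
; Debug prints report BeginPlay and show both axis values on screen.
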(event EventBeginPlay
  (Development|PrintString "BP BEGIN PLAY")
  (Class|TankMovementComponent|Initialise (Variables|Default|GetTankMovement) (Variables|Default|GetLeftTrack) (Variables|Default|GetRightTrack)))

(event Input|AxisEvents|InputAxisMoveForward
  (params (AxisValue :type Float%20%28single-precision%29))
  (Development|PrintString (Utilities|String|Append "ForwartThrottle" (Utilities|String|ToString(Float) AxisValue)) true false "(R=0.000000,G=0.660000,B=1.000000,A=1.000000)" 0.0)
  (Class|TankMovementComponent|IntendMoveForward (Variables|Default|GetTankMovement) AxisValue))

(event Input|AxisEvents|InputAxisTurnRight
  (params (AxisValue :type Float%20%28single-precision%29))
  (Development|PrintString (Utilities|String|Append "RightThrottle" (Utilities|String|ToString(Float) AxisValue)) true false "(R=0.000000,G=0.660000,B=1.000000,A=1.000000)" 0.0)
  (Class|TankMovementComponent|IntendTurnRight (Variables|Default|GetTankMovement) AxisValue (Input|AxisValues|GetMoveForward)))

(fn ConstructionScript)